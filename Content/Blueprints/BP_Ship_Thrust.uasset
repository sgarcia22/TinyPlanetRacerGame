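; Player-controlled ship Blueprint that flies with six degrees of freedom through physics impulses on ShipMesh.
; Throttle, strafe and lift axes push along the mesh's forward, right and up vectors.
; Roll, pitch and yaw axes apply angular impulses around those same local axes.
; Impulses are mass-dependent and applied on every axis event without delta-time scaling, so handling varies with frame rate.
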(event `InputAxis|IncreaseThrottle`
  (params (AxisValue :type "Float (single-precision)"))
  (bind _shipmesh (`self.ShipMesh`))
  ;[1 1 1] Thrust Forward/Backward
  (`PrimitiveComponent.AddImpulse` _shipmesh (* (`SceneComponent.GetForwardVector` _shipmesh) (* AxisValue 0.2)) "None" false))

(event `InputAxis|Roll`
  (params (AxisValue :type "Float (single-precision)"))
  (bind _shipmesh (`self.ShipMesh`))
  ;[1 1 1] Torque Up/Down - Roll
  (`PrimitiveComponent.AddAngularImpulseInRadians` _shipmesh (* (`SceneComponent.GetForwardVector` _shipmesh) (* AxisValue -0.1)) "None" false))

(event `InputAxis|MoveRight`
  (params (AxisValue :type "Float (single-precision)"))
  (bind _shipmesh (`self.ShipMesh`))
  ;[1 1 1] Thrust Left/Right
  (`PrimitiveComponent.AddImpulse` _shipmesh (* (`SceneComponent.GetRightVector` _shipmesh) (* AxisValue 0.2)) "None" false))

(event `InputAxis|Yaw`
  (params (AxisValue :type "Float (single-precision)"))
  (bind _shipmesh (`self.ShipMesh`))
  ;[1 1 1] Torque Left/Right - Yaw
  (`PrimitiveComponent.AddAngularImpulseInRadians` _shipmesh (* (`SceneComponent.GetUpVector` _shipmesh) (* AxisValue 0.1)) "None" false))

(event `InputAxis|MoveUp`
  (params (AxisValue :type "Float (single-precision)"))
  (bind _shipmesh (`self.ShipMesh`))
  ;[1 1 1] Thrust Up/Down
  (`PrimitiveComponent.AddImpulse` _shipmesh (* (`SceneComponent.GetUpVector` _shipmesh) (* AxisValue 0.2)) "None" false))

(event `InputAxis|Pitch`
  (params (AxisValue :type "Float (single-precision)"))
  (bind _shipmesh (`self.ShipMesh`))
  ;[1 1 1] Torque Left/Right - Yaw
  (`PrimitiveComponent.AddAngularImpulseInRadians` _shipmesh (* (`SceneComponent.GetRightVector` _shipmesh) (* AxisValue -0.1)) "None" false))

(fn `UserConstructionScript`)
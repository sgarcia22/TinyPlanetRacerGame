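; BaseShip is a player-controlled flying ship Blueprint with throttle, rotation and strafe movement.
; Throttle input eases a desired speed toward forward maximum or a tenth of it in reverse, and Tick interpolates current speed toward it to offset the actor locally.
; Yaw and Pitch apply delta-time-scaled local rotation.
; MoveRight strafes and rolls, while MoveUp strafes vertically with zero rotation; neither strafe offset is scaled by delta time.
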(event `self.ReceiveTick`
  (params (DeltaSeconds :type "Float (single-precision)"))
  ;[1 1 1] Tick - Move Forward/Backward
  (bind _output_get (set `self.CurrentSpeed` (`KismetMathLibrary.FInterpTo` (`self.CurrentSpeed`) (`self.DesiredSpeed`) (`GameplayStatics.GetWorldDeltaSeconds`) (/ (`self.AccelerationInterp`) 2.0))))
  (`self.K2_AddActorLocalOffset` (`KismetMathLibrary.MakeVector` _output_get)))

(event `InputAxis|IncreaseThrottle`
  (params (AxisValue :type "Float (single-precision)"))
  ;[1 1 1] Throttle
  (if (> AxisValue 0.0)
    (set `self.DesiredSpeed` (`KismetMathLibrary.FInterpTo` (`self.DesiredSpeed`) (`self.MaxSpeed`) (`GameplayStatics.GetWorldDeltaSeconds`) (`self.AccelerationInterp`)))
    (elif (< AxisValue 0.0)
      (set `self.DesiredSpeed` (`KismetMathLibrary.FInterpTo` (`self.DesiredSpeed`) (* (/ (`self.MaxSpeed`) 10.0) -1.0) (`GameplayStatics.GetWorldDeltaSeconds`) (`self.AccelerationInterp`))))))

(event `InputAxis|Yaw`
  (params (AxisValue :type "Float (single-precision)"))
  ;[1 1 1] Camera Rotation
  (if (!= AxisValue 0.0)
    (`self.K2_AddActorLocalRotation` (`KismetMathLibrary.MakeRotator` 0.0 0.0 (* (* AxisValue (`GameplayStatics.GetWorldDeltaSeconds`)) 51.0)))))

(event `InputAxis|Pitch`
  (params (AxisValue :type "Float (single-precision)"))
  ;[1 1 1] Camera Rotation
  (if (!= AxisValue 0.0)
    (`self.K2_AddActorLocalRotation` (`KismetMathLibrary.MakeRotator` 0.0 (* (* AxisValue (`GameplayStatics.GetWorldDeltaSeconds`)) 51.0)))))

(event `InputAxis|MoveRight`
  (params (AxisValue :type "Float (single-precision)"))
  ;[1 1 1] Strafing
  (`|ExecutionSequence`
    (:`then_0`
      (if (!= AxisValue 0.0)
        (`self.K2_AddActorLocalOffset` (`KismetMathLibrary.MakeVector` 0.0 (* AxisValue (`self.StrafeSpeed`))))))
    (:`then_1`
      (if (!= AxisValue 0.0)
        (`self.K2_AddActorLocalRotation` (`KismetMathLibrary.MakeRotator` (* (* AxisValue (`GameplayStatics.GetWorldDeltaSeconds`)) 51.0)))))))

(event `InputAxis|MoveUp`
  (params (AxisValue :type "Float (single-precision)"))
  (bind _returnvalue (!= AxisValue 0.0))
  ;[1 1 1] Strafing
  (`|ExecutionSequence`
    (:`then_0`
      (if _returnvalue
        (`self.K2_AddActorLocalOffset` (`KismetMathLibrary.MakeVector` 0.0 0.0 (* AxisValue (`self.StrafeSpeed`))))))
    (:`then_1`
      (if _returnvalue
        (`self.K2_AddActorLocalRotation` (`KismetMathLibrary.MakeRotator` 0.0))))))

(fn `UserConstructionScript`)
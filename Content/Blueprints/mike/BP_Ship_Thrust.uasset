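; Player-controlled ship with six-degree-of-freedom physics flight, where input axes apply velocity-change impulses to ShipMesh for thrust and rotation along its local axes.
; Tick adds speed-dependent drag: cubic for linear velocity, quadratic for angular, with only linear drag scaled by delta time.
; BeginPlay teleports the ship to the PlayerStart tagged with its PlayerInt.
; Fire only prints debug text, and SetColor, uncalled here, assigns player 1's material.
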(event `InputAction|Fire`
  (params (Key :type "Key Structure"))
  (:`Pressed`
    (`KismetSystemLibrary.PrintString` "Fire_THRUST")))

(event `self.ReceiveTick`
  (params (DeltaSeconds :type "Float (single-precision)"))
  (bind _shipmesh (`self.ShipMesh`))
  (bind _returnvalue (`SceneComponent.GetComponentVelocity` _shipmesh))
  (bind _returnvalue_2 (`PrimitiveComponent.GetPhysicsAngularVelocityInDegrees` (`self.ShipMesh`) "None"))
  (bind _returnvalue_3 (`KismetMathLibrary.VSize` _returnvalue_2))
  (`PrimitiveComponent.AddImpulse` _shipmesh (* (* _returnvalue (* DeltaSeconds -1e-05)) (`KismetMathLibrary.Square` (`KismetMathLibrary.VSize` _returnvalue))) "None" true)
  (`PrimitiveComponent.AddAngularImpulseInDegrees` (`self.ShipMesh`) (* (* _returnvalue_2 -0.001) _returnvalue_3) "None" true)
  (`KismetSystemLibrary.PrintString` (`KismetStringLibrary.Conv_DoubleToString` (`KismetMathLibrary.Square` _returnvalue_3))))

(event `self.ReceiveBeginPlay`
  ;[1 1 1] Spawn Multiple Players
  (`KismetSystemLibrary.PrintString` "SOPANWING")
  (`self.SpawnFunction`))

(event `InputAxis|Roll`
  (params (AxisValue :type "Float (single-precision)"))
  (bind _shipmesh (`self.ShipMesh`))
  ;[1 1 1] Torque Up/Down - Roll
  (`PrimitiveComponent.AddAngularImpulseInRadians` _shipmesh (* (`SceneComponent.GetForwardVector` _shipmesh) (* AxisValue (* -1 (`self.Rotation_multiplier`)))) "None" true))

(event `InputAxis|IncreaseThrottle`
  (params (AxisValue :type "Float (single-precision)"))
  (bind _shipmesh (`self.ShipMesh`))
  ;[1 1 1] Thrust Forward/Backward
  (`PrimitiveComponent.AddImpulse` _shipmesh (* (`SceneComponent.GetForwardVector` _shipmesh) (* AxisValue 2.0)) "None" true))

(event `InputAxis|MoveRight`
  (params (AxisValue :type "Float (single-precision)"))
  (bind _shipmesh (`self.ShipMesh`))
  ;[1 1 1] Thrust Left/Right
  (`PrimitiveComponent.AddImpulse` _shipmesh (* (`SceneComponent.GetRightVector` _shipmesh) (* AxisValue 2.0)) "None" true))

(event `InputAxis|Yaw`
  (params (AxisValue :type "Float (single-precision)"))
  (bind _shipmesh (`self.ShipMesh`))
  ;[1 1 1] Torque Left/Right - Yaw
  (`PrimitiveComponent.AddAngularImpulseInRadians` _shipmesh (* (`SceneComponent.GetUpVector` _shipmesh) (* AxisValue (* 1 (`self.Rotation_multiplier`)))) "None" true))

(event `InputAxis|Pitch`
  (params (AxisValue :type "Float (single-precision)"))
  (bind _shipmesh (`self.ShipMesh`))
  ;[1 1 1] Torque Left/Right - Yaw
  (`PrimitiveComponent.AddAngularImpulseInRadians` _shipmesh (* (`SceneComponent.GetRightVector` _shipmesh) (* AxisValue (* -1 (`self.Rotation_multiplier`)))) "None" true))

(event `InputAxis|MoveUp`
  (params (AxisValue :type "Float (single-precision)"))
  (bind _shipmesh (`self.ShipMesh`))
  ;[1 1 1] Thrust Up/Down
  (`PrimitiveComponent.AddImpulse` _shipmesh (* (`SceneComponent.GetUpVector` _shipmesh) (* AxisValue -2.0)) "None" true))

(fn `NewFunction_0`
  ;[1 1 1] Thrust Left/Right
)

(fn `SetColor`
  (switch `int` (`self.PlayerInt`)
    (:`1`
      (`PrimitiveComponent.SetMaterial` (`self.ShipMesh`) 0 "/Game/StarterContent/Materials/M_Wood_Walnut.M_Wood_Walnut"))))

(fn `SpawnFunction`
  (`KismetSystemLibrary.PrintString` "TESTING_S{AWN_BP_THRUST")
  (bind _outactors (`GameplayStatics.GetAllActorsOfClass` "/Script/Engine.PlayerStart"))
  (for _array_element _outactors
    (if (== (`PlayerStart.PlayerStartTag` _array_element) (`KismetStringLibrary.Conv_StringToName` (`KismetStringLibrary.Concat_StrStr` "Player" (`KismetStringLibrary.Conv_IntToString` (`self.PlayerInt`)))))
      (bind _output_get (set `self.SpawnLocation` (`self.GetTransform` _array_element)))
      (`self.K2_SetActorTransform` _output_get false true))))

(fn `UserConstructionScript`)
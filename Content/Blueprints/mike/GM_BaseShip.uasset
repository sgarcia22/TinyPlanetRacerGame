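; GM_BaseShip is a game mode that sets up local multiplayer ship play when the level begins.
; SpawnPlayers first creates local players by controller index over a range set by NPlayers.
; A second loop spawns a BP_Ship_Thrust at the world origin for each index, passes it that index as PlayerInt and has the matching player controller possess it.
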(event `self.ReceiveBeginPlay`
  (`self.SpawnPlayers`))

(fn `SpawnPlayers`
  (bind _n_players (`self.n_players`))
  (`KismetSystemLibrary.PrintString` "TESTING_S{AWN_GM_")
  (for _index (range (+ _n_players 1))
    ;[1 1 1] Add extra players to the game
    (`GameplayStatics.CreatePlayer` _index))
  ;[1 1 1] Spawn and Possess Actors
  (for _index_2 (range (+ _n_players 1))
    (bind _returnvalue (`|SpawnActorFromClass` "/Game/Blueprints/mike/BP_Ship_Thrust.BP_Ship_Thrust_C" (`KismetMathLibrary.MakeTransform` (0.0 0.0 0.0)) "Undefined" "OverrideRootScale" null _index_2 null))
    (`Controller.Possess` (`GameplayStatics.GetPlayerController` _index_2) _returnvalue)
    (`KismetSystemLibrary.PrintString` "Hello")))

(fn `UserConstructionScript`)